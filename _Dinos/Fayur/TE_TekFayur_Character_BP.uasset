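; Tek Fayur dino character Blueprint that registers the creature with an external tekevolved.com web API when it is set up as tamed.
; On the server only, BPSetupTamed builds a URL from the dino's short name and descriptive name and sends it through ShooterGameState's HTTP GET.
; The response delegate is bound after the request is sent, and its handler just prints the returned string.
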(event `self.BPSetupTamed`
  (params (bWasJustTamed :type Boolean))
  (`/Engine/EditorBlueprintResources/ActorMacros.Switch Has Authority`
    (:`Authority`
      (bind _asshootergamestate (cast `ShooterGameState` (`GameplayStatics.GetGameState`)))
      (`ShooterGameState.HTTPGetRequest` _asshootergamestate (`KismetStringLibrary.Concat_StrStr` "http://tekevolved.com/tekapi/registerdino?name=" (`KismetStringLibrary.Concat_StrStr` (`self.GetShortName`) (`KismetStringLibrary.Concat_StrStr` "&type=" (`KismetStringLibrary.Replace` (`self.GetDescriptiveName`) " ")))))
      (add `ShooterGameState.OnHTTPGetResponse` _asshootergamestate (delegate `OnHTTPGetProcessed__DelegateSignature_Event`)))))

(event `OnHTTPGetProcessed__DelegateSignature_Event`
  (params (bSuccess :type Boolean) (StringResult :type String))
  (`KismetSystemLibrary.PrintString` StringResult))

(fn `UserConstructionScript`
  (`parent.UserConstructionScript`))